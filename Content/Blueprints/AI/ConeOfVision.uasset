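; AI vision cone that builds a procedural mesh from EQS results and tracks a SeePlayer flag.
; Each tick it runs the VisionCone query and converts the hit locations into flat, actor-relative vertices with fan triangles from vertex zero.
; CreateCone rebuilds the colliding mesh section and zeroes its world rotation.
; The seen event sets SeePlayer, and ending overlap with the cone clears it after a short delay.
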(event `self.ReceiveTick`
  (params (DeltaSeconds :type "Float (single-precision)"))
  (bind _returnvalue (`EnvQueryManager.RunEQSQuery` "/Game/Blueprints/AI/VisionCone.VisionCone" self "AllMatching"))
  (add `EnvQueryInstanceBlueprintWrapper.OnQueryFinishedEvent` _returnvalue (delegate `MakeVisionCone`)))

(event `MakeVisionCone`
  (params (QueryInstance :type "EnvQueryInstanceBlueprintWrapper Object Reference") (QueryStatus :type "EEnvQueryStatus Enum" :default "Processing"))
  (bind _resultlocations (`EnvQueryInstanceBlueprintWrapper.GetQueryResultsAsLocations` QueryInstance))
  (bind _output_get (set `self.SightPoints` _resultlocations))
  (bind (_vertices _triangles) (`self.Convert Sight Points` _output_get))
  (`self.CreateCone` _vertices _triangles))

(event `self.ReceiveBeginPlay`
  (`KismetArrayLibrary.Array_Resize` (`self.Vertices`) 26))

(event `seen`
  (set `self.seePlayer` true))

(event `self.VisionCone.OnComponentEndOverlap`
  (params (OverlappedComponent :type "PrimitiveComponent Object Reference") (OtherActor :type "Actor Object Reference") (OtherComp :type "PrimitiveComponent Object Reference") (OtherBodyIndex :type Integer))
  (`KismetSystemLibrary.Delay` 0.1)
  (set `self.seePlayer` false))

(fn `Convert Sight Points`
  (params (SightPoints :type "Array of Vector Structure (by ref)"))
  (returns (Vertices :type "Array of Vector Structure") (Triangles :type "Array of Integer"))
  (bind _returnvalue (* (`KismetArrayLibrary.Array_Length` (`self.Vertices`)) 3))
  (`KismetArrayLibrary.Array_Set` (`self.Vertices`))
  (for (_array_element _array_index) SightPoints
    (`KismetArrayLibrary.Array_Set` (`self.Vertices`) _array_index (`KismetMathLibrary.MakeVector` (- (.x _array_element) (.x (`self.K2_GetActorLocation`))) (- (.y _array_element) (.y (`self.K2_GetActorLocation`))))))
  (`KismetArrayLibrary.Array_Resize` (`self.Triangles`) _returnvalue)
  (for _index (range (+ _returnvalue 1))
    (bind _returnvalue_2 (* _index 3))
    (`KismetArrayLibrary.Array_Set` (`self.Triangles`) _returnvalue_2)
    (bind _returnvalue_3 (+ _returnvalue_2 1))
    (bind _returnvalue_4 (+ _index 1))
    (`KismetArrayLibrary.Array_Set` (`self.Triangles`) _returnvalue_3 _returnvalue_4)
    (`KismetArrayLibrary.Array_Set` (`self.Triangles`) (+ _returnvalue_3 1) (+ _returnvalue_4 1)))
  (return (`self.Vertices`) (`self.Triangles`)))

(fn `CreateCone`
  (params (Vertices :type "Array of Vector Structure (by ref)") (Triangles :type "Array of Integer (by ref)"))
  (bind _visioncone (`self.VisionCone`))
  (`ProceduralMeshComponent.CreateMeshSection_LinearColor` :`self` _visioncone :`Vertices` Vertices :`Triangles` Triangles :`bCreateCollision` true)
  (`PrimitiveComponent.SetMaterial` _visioncone 0 "/Game/Arts/Meshes/FBX/lambert1.lambert1")
  (`SceneComponent.K2_SetWorldRotation` :`self` _visioncone))

(fn `UserConstructionScript`)