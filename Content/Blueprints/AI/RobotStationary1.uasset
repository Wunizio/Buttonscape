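; Stationary robot AI that detects the player through attached vision cones and holds that awareness briefly after losing sight.
; On BeginPlay it spawns a ConeOfVision actor, attaches it to its VisionCone component and stores it in a list.
; Tick polls each cone, setting SeePlayer and a paused reset timer while the player is visible.
; When sight is lost, it prints a debug string and resumes the timer that clears SeePlayer.
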(event `self.ReceiveTick`
  (params (DeltaSeconds :type "Float (single-precision)"))
  (for _array_element (`self.VisionConeList`)
    (`/Engine/EditorBlueprintResources/StandardMacros.IsValid` _array_element
      (:`Is Valid`
        (if (`/Game/Blueprints/AI/ConeOfVision.seePlayer` _array_element)
          (set `self.SeePlayer` true)
          (bind _returnvalue (`KismetSystemLibrary.K2_SetTimerDelegate` (delegate `Reset`) 5.0))
          (`KismetSystemLibrary.K2_PauseTimerHandle` _returnvalue)
          (elif (`self.SeePlayer`)
            (`KismetSystemLibrary.PrintString` "SS")
            (`KismetSystemLibrary.K2_UnPauseTimerHandle` _returnvalue)))))))

(event `Reset`
  (set `self.SeePlayer` false))

(event `self.ReceiveBeginPlay`
  (`self.CreateVisionCone` (`self.VisionCone`)))

(fn `CreateVisionCone`
  (params (Attacher :type "StaticMeshComponent Object Reference"))
  (bind _returnvalue (`|SpawnActorFromClass` "/Game/Blueprints/AI/ConeOfVision.ConeOfVision_C" (`KismetMathLibrary.MakeTransform` (0.0 0.0 0.0)) "Undefined" "OverrideRootScale" null null))
  (`KismetArrayLibrary.Array_Add` (`self.VisionConeList`) _returnvalue)
  (`self.K2_AttachToComponent` _returnvalue Attacher "None" "KeepRelative" "KeepRelative" "KeepRelative" true))

(fn `UserConstructionScript`)