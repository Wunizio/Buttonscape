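; WButton is a pressable button Blueprint that moves linked walls when triggered.
; ButtonReact clears the player FPCharacter's CanBePressed flag, plays a beep, and runs the Press timeline, which nudges the button mesh along local Z.
; When the timeline finishes, it loops over the Wall array and calls MoveWall on each entry.
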(event `ButtonReact`
  (bind _staticmeshcomponent (`self.StaticMeshComponent`))
  ;[1 1 1] Button React
  (bind _asfpcharacter (cast `/Game/Blueprints/FPCharacter` (`GameplayStatics.GetPlayerPawn` 0)))
  (set `/Game/Blueprints/FPCharacter.canBePressed` false _asfpcharacter)
  (`GameplayStatics.PlaySoundAtLocation` "/Game/Arts/sounds/ButtonGoBeepV1.ButtonGoBeepV1" (`SceneComponent.K2_GetComponentLocation` _staticmeshcomponent) (struct) 1.0 1.0 0.0 null null null)
  (bind (_direction _press) (`Timeline|Press` :!via `PlayFromStart`)
    (:`Update`
      (`SceneComponent.K2_AddRelativeLocation` _staticmeshcomponent (`KismetMathLibrary.MakeVector` 0.0 0.0 _press) false false))
    (:`Finished`
      (for _array_element (`self.Wall`)
        (bind _aswall (cast `/Game/Blueprints/Wall` _array_element))
        (`/Game/Blueprints/Wall.MoveWall` _aswall)))))

(fn `UserConstructionScript`)